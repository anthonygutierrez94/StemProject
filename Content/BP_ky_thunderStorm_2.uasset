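; BP_ky_thunderStorm_2 is a lightning storm actor, apparently an unfinished hazard meant to damage Forge actors.
; Cylinder hits only print the other actor's name on authority, and the particle overlap leads to an empty authority switch.
; A custom event spawns the lightning emitter at the actor's location.
; The chain that damages a Forge, plays the particle, unhides the actor and destroys it after a short delay is disconnected and never runs.
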(event OnComponentBeginOverlap(ParticleSystem)
  (params (OverlappedComponent :type Primitive%20Component%20Object%20Reference) (OtherActor :type Actor%20Object%20Reference) (OtherComp :type Primitive%20Component%20Object%20Reference) (OtherBodyIndex :type Integer) (bFromSweep :type Boolean) (SweepResult :type Hit%20Result%20Structure%20%28by%20ref%29))
  (Networking|SwitchHasAuthority))

(event OnComponentHit(Cylinder)
  (params (HitComponent :type Primitive%20Component%20Object%20Reference) (OtherActor :type Actor%20Object%20Reference) (OtherComp :type Primitive%20Component%20Object%20Reference) (NormalImpulse :type Vector :default "0, 0, 0") (Hit :type Hit%20Result%20Structure%20%28by%20ref%29))
  (Networking|SwitchHasAuthority
    (:Authority
      (Development|PrintString (Utilities|GetDisplayName OtherActor)))))

(event Custom|Multi_playParticle
  (Effects|SpawnEmitteratLocation "/Game/FXVarietyPack/Particles/P_ky_lightning3.P_ky_lightning3" (Transformation|GetActorLocation)))

(event EventBeginPlay
  (|CallParentFunction) ; This node is disabled and will not be called.\nDrag off pins to build functionality.
)

(event Collision|EventActorBeginOverlap
  (params (OtherActor :type Actor%20Object%20Reference))
  (|CallParentFunction OtherActor) ; This node is disabled and will not be called.\nDrag off pins to build functionality.
)

(event EventTick
  (params (DeltaSeconds :type Float%20%28single-precision%29))
  (|CallParentFunction DeltaSeconds) ; This node is disabled and will not be called.\nDrag off pins to build functionality.
)

(fn ConstructionScript
  (|CallParentFunction))