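; BP_FireBall is a fireball actor that damages Forge actors it overlaps.
; On the server, a Sphere overlap with a Forge applies fixed damage, calls Multi_playParticle to spawn an explosion, then hides the fireball.
; A short delay precedes destruction of the hidden actor.
; Sphere hits only print the other actor's name on the server, and the overlap also prints a debug message.
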(event OnComponentBeginOverlap(Sphere)
  (params (OverlappedComponent :type Primitive%20Component%20Object%20Reference) (OtherActor :type Actor%20Object%20Reference) (OtherComp :type Primitive%20Component%20Object%20Reference) (OtherBodyIndex :type Integer) (bFromSweep :type Boolean) (SweepResult :type Hit%20Result%20Structure%20%28by%20ref%29))
  (Networking|SwitchHasAuthority
    (:Authority
      (bind _asforge (Utilities|Casting|CastToForge OtherActor))
      (Utilities|IsValid _asforge
        (:Is%20Valid
          (Development|PrintString "Hello")
          (Game|Damage|ApplyDamage _asforge 1e+01 0 0)
          (CallFunction|MultiPlayParticle)
          (Rendering|SetActorHiddenInGame true)
          (Utilities|FlowControl|Delay 0.2)
          (Actor|DestroyActor))))))

(event OnComponentHit(Sphere)
  (params (HitComponent :type Primitive%20Component%20Object%20Reference) (OtherActor :type Actor%20Object%20Reference) (OtherComp :type Primitive%20Component%20Object%20Reference) (NormalImpulse :type Vector :default "0, 0, 0") (Hit :type Hit%20Result%20Structure%20%28by%20ref%29))
  (Networking|SwitchHasAuthority
    (:Authority
      (Development|PrintString (Utilities|GetDisplayName OtherActor)))))

(event Custom|Multi_playParticle
  (Effects|SpawnEmitteratLocation "/Game/FXVarietyPack/Particles/P_ky_explosion.P_ky_explosion" (Transformation|GetActorLocation)))

(event EventBeginPlay)

(event Collision|EventActorBeginOverlap
  (params (OtherActor :type Actor%20Object%20Reference)))

(event EventTick
  (params (DeltaSeconds :type Float%20%28single-precision%29)))

(fn ConstructionScript)