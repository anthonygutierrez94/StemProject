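; Forge is a character Blueprint that shoots fireballs on player input and reports damage it receives.
; The ShootFireball press calls an SRV-prefixed event, named as a server call, which always spawns BP_FireBall regardless of collision.
; The spawn point is the actor location plus the forward vector with 40 added to it, rather than scaled by 40.
; AnyDamage only prints the damage amount.
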(event Custom|SRV_ShootFireball
  (Game|SpawnActorfromClass "/Game/BP_FireBall.BP_FireBall_C" (Math|Transform|MakeTransform (+ (Transformation|GetActorLocation) (+ (Transformation|GetActorForwardVector) 4e+01)) "0, 0, 0" "1,1,1") "AlwaysSpawn" 0 0))

(event EventBeginPlay)

(event Collision|EventActorBeginOverlap
  (params (OtherActor :type Actor%20Object%20Reference)))

(event EventTick
  (params (DeltaSeconds :type Float%20%28single-precision%29)))

(event Game|Damage|EventAnyDamage
  (params (Damage :type Float%20%28single-precision%29) (DamageType :type Damage%20Type%20Object%20Reference) (InstigatedBy :type Controller%20Object%20Reference) (DamageCauser :type Actor%20Object%20Reference))
  (Development|PrintString (Utilities|String|ToString(Float) Damage)))

(event Input|ActionEvents|InputActionShootFireball
  (params (Key :type Key%20Structure :default "None"))
  (:Pressed
    (CallFunction|SRVShootFireball)))

(fn ConstructionScript
  (|CallParentFunction))